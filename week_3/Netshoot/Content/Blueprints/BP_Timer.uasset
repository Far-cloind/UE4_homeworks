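; BP_Timer is a spawner actor that periodically creates BP_ScoreCube actors during play.
; After a short delay on BeginPlay, it starts a looping timer that fires CreateScoreCube every second.
; Each cube spawns at Y zero on a randomly chosen side, using a random bool to flip between mirrored X positions, with a random height.
; Spawn collision handling adjusts the location if possible but always spawns.
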(event `self.ReceiveBeginPlay`
  (`KismetSystemLibrary.Delay` 1.0)
  (`KismetSystemLibrary.K2_SetTimerDelegate` (delegate `CreateScoreCube`) 1.0 true))

(event `CreateScoreCube`
  (`|SpawnActorFromClass` "/Game/Blueprints/BP_ScoreCube.BP_ScoreCube_C" (`KismetMathLibrary.Conv_VectorToTransform` (`KismetMathLibrary.MakeVector` (`KismetMathLibrary.Conv_IntToDouble` (- 850 (* 1700 (`KismetMathLibrary.Conv_BoolToInt` (`KismetMathLibrary.RandomBool`))))) 0.0 (`KismetMathLibrary.RandomFloatInRange` 70.0 450.0))) "AdjustIfPossibleButAlwaysSpawn" "OverrideRootScale" null null))

(fn `UserConstructionScript`)