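; Grenade launcher projectile that bounces or explodes depending on the surface it hits.
; On Hit it identifies the surface by the name of the other component's first material, then either sets projectile bounciness high or near zero, or destroys itself.
; EndPlay spawns the hit particle effect at the mesh location and plays a 2D explosion sound, with no damage logic in the graph.
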(event `self.ReceiveHit`
  (params (MyComp :type "PrimitiveComponent Object Reference") (Other :type "Actor Object Reference") (OtherComp :type "PrimitiveComponent Object Reference") (bSelfMoved :type Boolean) (HitLocation :type "Vector Structure") (HitNormal :type "Vector Structure") (NormalImpulse :type "Vector Structure") (Hit :type "HitResult Structure (by ref)"))
  (bind _returnvalue (`KismetSystemLibrary.GetObjectName` (`PrimitiveComponent.GetMaterial` OtherComp 0)))
  (if (`KismetStringLibrary.EqualEqual_StrStr` "M_Player_Inst" _returnvalue)
    (set `ProjectileMovementComponent.Bounciness` 0.8 (`self.ProjectileMovement`))
    (elif (`KismetStringLibrary.EqualEqual_StrStr` "M_Player" _returnvalue)
      (set `ProjectileMovementComponent.Bounciness` 0.01 (`self.ProjectileMovement`))
      (elif (`KismetStringLibrary.EqualEqual_StrStr` "M_Basic_2" _returnvalue)
        (`self.K2_DestroyActor`)
        (elif (`KismetStringLibrary.EqualEqual_StrStr` "Soldier_body1" _returnvalue)
          (`self.K2_DestroyActor`))))))

(event `self.ReceiveEndPlay`
  (params (EndPlayReason :type "EEndPlayReason Enum" :default "Destroyed"))
  (`GameplayStatics.SpawnEmitterAtLocation` "/Game/Effects/P_Hit.P_Hit" (`SceneComponent.K2_GetComponentLocation` (`self.StaticMesh`)) (struct) (690.0 1.0 1.0))
  (`GameplayStatics.PlaySound2D` "/Game/Audio/explosion2.explosion2" 1.0 1.0 0.0 null null)
  (`KismetSystemLibrary.Delay` 0.5))

(fn `UserConstructionScript`)