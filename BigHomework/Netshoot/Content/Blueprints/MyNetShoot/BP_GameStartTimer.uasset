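; BP_GameStartTimer runs the pre-match countdown for the NetShoot game mode.
; RefreshStartTimer restarts a timeline on the authority that drives StartTime, then calls GameStart on the game mode and ClientHideStartTimer when it finishes.
; Tick copies the truncated StartTime into the first player controller's start timer widget, and ClientHideStartTimer hides that widget.
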(event `RefreshStartTimer`
  (`/Engine/EditorBlueprintResources/ActorMacros.Switch Has Authority`
    (:`Authority`
      (bind (_direction `_新建轨道_0`) (`Timeline|时间轴_0` :!via `PlayFromStart`)
        (:`Update`
          (set `self.StartTime` `_新建轨道_0`)
          (bind _asmy_game_mode_netshoot (cast `/Game/Blueprints/MyNetShoot/MyGameMode_Netshoot` (`GameplayStatics.GetGameMode`))))
        (:`Finished`
          (`/Game/Blueprints/MyNetShoot/MyGameMode_Netshoot.GameStart` _asmy_game_mode_netshoot)
          (`self.ClientHideStartTimer`))))))

(event `self.ReceiveTick`
  (params (DeltaSeconds :type "Float (single-precision)"))
  (bind _asmy_player_controller_netshoot (cast `/Game/Blueprints/MyNetShoot/MyPlayerController_Netshoot` (`GameplayStatics.GetPlayerController` 0)))
  (set `/Game/Blueprints/MyNetShoot/Widgets/StartTimerWidget.TimeRemain` (`KismetMathLibrary.FTrunc` (`self.StartTime`)) (`/Game/Blueprints/MyNetShoot/MyPlayerController_Netshoot.StartTimerWidget` _asmy_player_controller_netshoot)))

(event `ClientHideStartTimer`
  (bind _asmy_player_controller_netshoot (cast `/Game/Blueprints/MyNetShoot/MyPlayerController_Netshoot` (`GameplayStatics.GetPlayerController` 0)))
  (`/Game/Blueprints/MyNetShoot/MyPlayerController_Netshoot.HideStartTimerWidget` _asmy_player_controller_netshoot))

(fn `UserConstructionScript`)