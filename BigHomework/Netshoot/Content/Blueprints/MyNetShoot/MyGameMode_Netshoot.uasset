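; Game mode for the Netshoot multiplayer game, managing player joins, respawns, match start and the win settlement.
; Pre-start logins register controllers, assign player numbers for consistent scoreboard order and refresh a shared start timer.
; Respawning replaces the player's pawn with a new character at a random reachable navigation point around a lazily spawned Michelle actor.
; Game start spawns the destination and removes the timer; a win tells every registered controller to show settlement.
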(event `RespawnPlayerEvent`
  (params (PlayerController :type "PlayerController Object Reference"))
  (bind _returnvalue (`Controller.K2_GetPawn` PlayerController))
  (bind _michelle (`self.Michelle`))
  ;[1 1 1] Respawns the player
  (`/Engine/EditorBlueprintResources/StandardMacros.IsValid` _returnvalue
    (:`Is Valid`
      (`self.K2_DestroyActor` _returnvalue))
    (:`Is Not Valid`
      _))
  (`/Engine/EditorBlueprintResources/StandardMacros.IsValid` _michelle
    (:`Is Valid`
      _)
    (:`Is Not Valid`
      (bind _returnvalue_2 (`|SpawnActorFromClass` "/Game/Characters/Michelle/BP_Michelle.BP_Michelle_C" (`KismetMathLibrary.MakeTransform` (-110.0 -700.0 88.0) (struct :`Yaw` 90.0)) "AdjustIfPossibleButAlwaysSpawn" "OverrideRootScale" null null))
      (set `self.Michelle` _returnvalue_2)))
  (bind _returnvalue_3 (`|SpawnActorFromClass` "/Game/Characters/Soldier/BP_MyCharacter.BP_MyCharacter_C" (`KismetMathLibrary.Conv_VectorToTransform` (`NavigationSystemV1.K2_GetRandomReachablePointInRadius` (`self.K2_GetActorLocation` _michelle) 300.0 null null)) "AdjustIfPossibleButDontSpawnIfColliding" "OverrideRootScale" null null))
  (`Controller.Possess` PlayerController _returnvalue_3)
  (bind _asmy_player_controller_netshoot (cast `/Game/Blueprints/MyNetShoot/MyPlayerController_Netshoot` PlayerController))
  (`/Game/Blueprints/MyNetShoot/MyPlayerController_Netshoot.ClientUpdateMyCharacter` _asmy_player_controller_netshoot))

(event `self.K2_PostLogin`
  (params (NewPlayer :type "PlayerController Object Reference"))
  (bind _starttimer (`self.StartTimer`))
  ;[1 1 1] Post login
  (if (not (`self.IsGameStarted`))
    (bind _asmy_player_controller_netshoot (cast `/Game/Blueprints/MyNetShoot/MyPlayerController_Netshoot` NewPlayer))
    (`KismetArrayLibrary.Array_Add` (`self.AllMyPlayerController`) _asmy_player_controller_netshoot)
    (bind _asmy_player_state (cast `/Game/Blueprints/MyPlayerState` (`Controller.PlayerState` NewPlayer)))
    (set `/Game/Blueprints/MyPlayerState.PlayerNumber` (`KismetArrayLibrary.Array_Length` (`GameState.PlayerArray` (`GameplayStatics.GetGameState`))) _asmy_player_state) ; Makes the scoreboard in the same order for all players
    (bind _asmy_player_controller_netshoot_2 (cast `/Game/Blueprints/MyNetShoot/MyPlayerController_Netshoot` NewPlayer))
    (`/Game/Blueprints/MyNetShoot/MyPlayerController_Netshoot.ClientPostLogin` _asmy_player_controller_netshoot_2)
    (`/Engine/EditorBlueprintResources/StandardMacros.IsValid` _starttimer
      (:`Is Valid`
        _)
      (:`Is Not Valid`
        (bind _returnvalue (`|SpawnActorFromClass` "/Game/Blueprints/MyNetShoot/BP_GameStartTimer.BP_GameStartTimer_C" (`KismetMathLibrary.Conv_VectorToTransform` (-170.0 -3200.0 0.0)) "AdjustIfPossibleButAlwaysSpawn" "OverrideRootScale" null null))
        (set `self.StartTimer` _returnvalue)))
    (`/Game/Blueprints/MyNetShoot/BP_GameStartTimer.RefreshStartTimer` _starttimer)
    (set `self.IsGameStarted` false)))

(event `GameStart`
  ;[1 1 1] 游戏开始
  (bind _returnvalue (`|SpawnActorFromClass` "/Game/Blueprints/MyNetShoot/BP_Destination.BP_Destination_C" (`KismetMathLibrary.Conv_VectorToTransform` (-170.0 -3200.0 0.0)) "AdjustIfPossibleButAlwaysSpawn" "OverrideRootScale" null null))
  (set `self.Destination` _returnvalue)
  (set `self.IsGameStarted` true)
  (`self.K2_DestroyActor` (`self.StartTimer`)))

(event `PlayerWinEvent`
  ;[1 1 1] Broadcast to all PC to open their settlement
  (for _array_element (`self.AllMyPlayerController`)
    (`/Game/Blueprints/MyNetShoot/MyPlayerController_Netshoot.ShowSettlement` _array_element)))

(fn `UserConstructionScript`)