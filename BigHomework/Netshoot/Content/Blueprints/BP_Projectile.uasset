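; Projectile actor that damages the characters it hits and destroys itself on impact.
; The Hit event runs a cast chain over BP_MyCharacter, BP_Mutant and BP_Michelle, applying damage credited to the instigator's controller, slightly higher for the Mutant.
; Each match plays a pitch-randomized sound, but only the BP_MyCharacter branch passes the hit location to it.
; Any hit, matched or not, destroys the projectile and spawns a hit particle effect.
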(event `self.ReceiveHit`
  (params (MyComp :type "PrimitiveComponent Object Reference") (Other :type "Actor Object Reference") (OtherComp :type "PrimitiveComponent Object Reference") (bSelfMoved :type Boolean) (HitLocation :type "Vector Structure") (HitNormal :type "Vector Structure") (NormalImpulse :type "Vector Structure") (Hit :type "HitResult Structure (by ref)"))
  (cast `/Game/Characters/Soldier/BP_MyCharacter` Other
    (:`then`
      ;[1 1 1] Hit Character
      (`GameplayStatics.ApplyDamage` Other 30.0 (`self.GetInstigatorController`) self)
      (`GameplayStatics.PlaySoundAtLocation` "/Game/Sounds/SoundCue_Attentuated.SoundCue_Attentuated" HitLocation (struct) 1.0 (`KismetMathLibrary.RandomFloatInRange` 0.8 1.2) 0.0 null null null))
    (:`CastFailed`
      (bind _asbp_mutant (cast `/Game/Characters/Mutant/BP_Mutant` Other)
        (:`then`
          ;[1 1 1] Hit Mutant
          (`GameplayStatics.ApplyDamage` _asbp_mutant 35.0 (`self.GetInstigatorController`) self)
          (`GameplayStatics.PlaySoundAtLocation` "/Game/Audio/RifleHit_Cue.RifleHit_Cue" (0.0 0.0 0.0) (struct) 0.3 (`KismetMathLibrary.RandomFloatInRange` 0.8 1.2) 0.0 null null null))
        (:`CastFailed`
          (bind _asbp_michelle (cast `/Game/Characters/Michelle/BP_Michelle` Other)
            (:`then`
              ;[1 1 1] Hit Michelle
              (`GameplayStatics.ApplyDamage` _asbp_michelle 30.0 (`self.GetInstigatorController`) self)
              (`GameplayStatics.PlaySoundAtLocation` "/Game/Sounds/SoundCue_Attentuated.SoundCue_Attentuated" (0.0 0.0 0.0) (struct) 1.0 (`KismetMathLibrary.RandomFloatInRange` 0.8 1.2) 0.0 null null null))
            (:`CastFailed`
              _))))))
  (`self.K2_DestroyActor`)
  (`GameplayStatics.SpawnEmitterAtLocation` "/Game/Effects/P_Hit.P_Hit" HitLocation))

(fn `UserConstructionScript`)