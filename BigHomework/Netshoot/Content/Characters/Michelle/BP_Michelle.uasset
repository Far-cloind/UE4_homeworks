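; BP_Michelle is the Michelle NPC, with health and an overhead health bar widget.
; On BeginPlay it sets the HeadHealthBar's name label and tints its fill purple.
; AnyDamage subtracts truncated damage from CurrentHealth, updates the bar and clears IsAlive at zero or below.
; UpdateHeadUI sets the bar's maximum, then uses a timeline to ease the displayed health toward the new value.
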(event `self.ReceiveBeginPlay`
  (bind _ashead_health_bar (cast `/Game/Blueprints/MyNetShoot/Widgets/HeadHealthBar` (`WidgetComponent.GetWidget` (`self.PlayerHeadHealthBar`))))
  (`TextBlock.SetText` (`/Game/Blueprints/MyNetShoot/Widgets/HeadHealthBar.Name` _ashead_health_bar) "Michelle(NPC)")
  (bind _healthbar (`/Game/Blueprints/MyNetShoot/Widgets/HeadHealthBar.HealthBar` _ashead_health_bar))
  (bind (_widgetstyle_backgroundimage _widgetstyle_fillimage _widgetstyle_marqueeimage) (break `ProgressBarStyle` (`ProgressBar.WidgetStyle` _healthbar)))
  (bind (_imagesize _margin _tintcolor _resourceobject _drawas _tiling _mirroring) (break `SlateBrush` _widgetstyle_fillimage))
  (set `ProgressBar.WidgetStyle` (make `ProgressBarStyle` _widgetstyle_backgroundimage (make `SlateBrush` _imagesize _margin (make `SlateColor` (struct :`R` 0.615391 :`B` 1.0 :`A` 1.0)) _resourceobject _drawas _tiling _mirroring) _widgetstyle_marqueeimage) _healthbar))

(event `self.ReceiveAnyDamage`
  (params (Damage :type "Float (single-precision)") (DamageType :type "DamageType Object Reference") (InstigatedBy :type "Controller Object Reference") (DamageCauser :type "Actor Object Reference"))
  (if true
    (bind _output_get (set `self.CurrentHealth` (- (`self.CurrentHealth`) (`KismetMathLibrary.FTrunc` Damage))))
    (`self.UpdateHeadUI` _output_get (`self.MaxHealth`))
    (if (<= _output_get 0)
      (set `self.IsAlive` false))))

(event `UpdateHeadUI`
  (params (NewHealth :type Integer) (NewMaxHealth :type Integer))
  (bind _ashead_health_bar (cast `/Game/Blueprints/MyNetShoot/Widgets/HeadHealthBar` (`WidgetComponent.GetWidget` (`self.PlayerHeadHealthBar`))))
  (set `/Game/Blueprints/MyNetShoot/Widgets/HeadHealthBar.HeadUIMaxHealth` NewMaxHealth _ashead_health_bar)
  (bind (_direction _health) (`Timeline|时间轴_0` :!via `PlayFromStart`)
    (:`Update`
      (set `/Game/Blueprints/MyNetShoot/Widgets/HeadHealthBar.HeadUICurrentHealth` (`KismetMathLibrary.FTrunc` (+ (* NewHealth _health) (* (`/Game/Blueprints/MyNetShoot/Widgets/HeadHealthBar.HeadUICurrentHealth` _ashead_health_bar) (- 1.0 _health)))) _ashead_health_bar))))

(fn `UserConstructionScript`)