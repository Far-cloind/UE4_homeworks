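; AI controller for the Mutant character that runs its behavior tree and handles melee damage against its target.
; On possess it starts BT_Mutant with the NotArrive blackboard flag set to true.
; Every tick it compares pawn and Target positions, clearing NotArrive within punch range and setting it otherwise.
; The PunchDamage event applies fixed damage to the blackboard Target, passing that target as the damage causer.
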(event `self.ReceivePossess`
  (params (PossessedPawn :type "Pawn Object Reference"))
  (`self.RunBehaviorTree` "/Game/Characters/Mutant/BT_Mutant.BT_Mutant")
  (`BlackboardComponent.SetValueAsBool` (`self.Blackboard`) (`self.NotArrive`) true))

(event `self.ReceiveTick`
  (params (DeltaSeconds :type "Float (single-precision)"))
  (bind _asactor (cast `Actor` (`BlackboardComponent.GetValueAsObject` (`AIBlueprintHelperLibrary.GetBlackboard` null) "Target")))
  (if (<= (`KismetMathLibrary.Vector_Distance` (`self.K2_GetActorLocation` (`self.K2_GetPawn`)) (`self.K2_GetActorLocation` _asactor)) 150.0)
    (`BlackboardComponent.SetValueAsBool` (`AIBlueprintHelperLibrary.GetBlackboard` null) (`self.NotArrive`) false)
    (else
      (`BlackboardComponent.SetValueAsBool` (`AIBlueprintHelperLibrary.GetBlackboard` null) (`self.NotArrive`) true))))

(event `PunchDamage`
  (bind _asactor (cast `Actor` (`BlackboardComponent.GetValueAsObject` (`AIBlueprintHelperLibrary.GetBlackboard` null) "Target")))
  (`GameplayStatics.ApplyDamage` _asactor 15.0 self _asactor))

(fn `UserConstructionScript`)