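; BP_TrainingTimer is an actor that counts down the time limit of the training level.
; On BeginPlay it starts a looping one-second timer that calls CountSecond.
; Each tick increments CountNum on MyGameMode_Training, and when it reaches TotalTime it fires the game mode's TimeOutEvent and destroys the timer actor.
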(event `self.ReceiveBeginPlay`
  (`KismetSystemLibrary.K2_SetTimer` null "CountSecond" 1.0 true))

(fn `CountSecond`
  (bind _asmy_game_mode_training (cast `/Game/Blueprints/TrainingLevelBP/MyGameMode_Training` (`GameplayStatics.GetGameMode`)))
  (bind _result (`/Engine/EditorBlueprintResources/StandardMacros.IncrementInt` (`/Game/Blueprints/TrainingLevelBP/MyGameMode_Training.CountNum` _asmy_game_mode_training))
    (:`  `
      (if (== _result (`/Game/Blueprints/TrainingLevelBP/MyGameMode_Training.TotalTime` _asmy_game_mode_training))
        (`/Game/Blueprints/TrainingLevelBP/MyGameMode_Training.TimeOutEvent` _asmy_game_mode_training)
        (`self.K2_DestroyActor`)))))

(fn `UserConstructionScript`)