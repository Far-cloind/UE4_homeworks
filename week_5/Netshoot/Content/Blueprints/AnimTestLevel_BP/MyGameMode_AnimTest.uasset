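; Game mode for the animation test level that sets up the session at start and handles player respawning.
; On BeginPlay it spawns a BP_Timer actor at the origin and calls ClientPostLogin on the first player's animation-test controller.
; RespawnPlayerEvent destroys the controller's current pawn, if valid, then spawns a MyCharacter_BP at the first PlayerStart found and possesses it.
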(event `RespawnPlayerEvent`
  (params (PlayerController :type "PlayerController Object Reference"))
  (bind _returnvalue (`Controller.K2_GetPawn` PlayerController))
  ;[1 1 1] Respawns the player
  (`/Engine/EditorBlueprintResources/StandardMacros.IsValid` _returnvalue
    (:`Is Valid`
      (`self.K2_DestroyActor` _returnvalue)
      (bind _outactors (`GameplayStatics.GetAllActorsOfClass` "/Script/Engine.PlayerStart"))
      (bind _returnvalue_2 (`|SpawnActorFromClass` "/Game/Characters/MyCharacter_BP.MyCharacter_BP_C" (`self.GetTransform` (`|GetArrayItem` _outactors)) "AdjustIfPossibleButDontSpawnIfColliding" "OverrideRootScale" null null))
      (`Controller.Possess` PlayerController _returnvalue_2))))

(event `self.ReceiveBeginPlay`
  ;[1 1 1] Create Timer
  (`|SpawnActorFromClass` "/Game/Blueprints/BP_Timer.BP_Timer_C" (`KismetMathLibrary.Conv_VectorToTransform` (0.0 0.0 0.0)) "AdjustIfPossibleButAlwaysSpawn" "OverrideRootScale" null null)
  (bind _asmy_player_controller_animation_test (cast `/Game/Blueprints/AnimTestLevel_BP/MyPlayerController_AnimationTest` (`GameplayStatics.GetPlayerController` 0)))
  (`/Game/Blueprints/AnimTestLevel_BP/MyPlayerController_AnimationTest.ClientPostLogin` _asmy_player_controller_animation_test))

(fn `UserConstructionScript`)