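; BP_ScoreCube is a moving target cube that awards a point to the player who damages it.
; On BeginPlay it picks one of two timelines by the sign of its X position, driving only X while keeping Y and Z, then destroys itself when the timeline finishes.
; Any damage destroys the cube and calls IncrementScore on the instigator's MyPlayerState.
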(event `self.ReceiveBeginPlay`
  ;[1 1 1] Set Cube Movement
  (if (> (.x (.location (`self.GetTransform`))) 0.0)
    (bind (_direction `_新建轨道_0`) (`Timeline|timeline1`)
      (:`Update`
        (`self.K2_SetActorLocation` (`KismetMathLibrary.MakeVector` `_新建轨道_0` (.y (.location (`self.GetTransform`))) (.z (.location (`self.GetTransform`))))))
      (:`Finished`
        (`self.K2_DestroyActor` :!label _label)))
    (else
      (bind (_direction_2 `_新建轨道_0_2`) (`Timeline|timeline2`)
        (:`Update`
          (`self.K2_SetActorLocation` (`KismetMathLibrary.MakeVector` `_新建轨道_0_2` (.y (.location (`self.GetTransform`))) (.z (.location (`self.GetTransform`))))))
        (:`Finished`
          (goto _label))))))

(event `self.ReceiveAnyDamage`
  (params (Damage :type "Float (single-precision)") (DamageType :type "DamageType Object Reference") (InstigatedBy :type "Controller Object Reference") (DamageCauser :type "Actor Object Reference"))
  ;[1 1 1] Increment Score
  (`self.K2_DestroyActor`)
  (bind _asmy_player_state (cast `/Game/Blueprints/MyPlayerState` (`Controller.PlayerState` InstigatedBy)))
  (`/Game/Blueprints/MyPlayerState.IncrementScore` _asmy_player_state))

(fn `UserConstructionScript`)