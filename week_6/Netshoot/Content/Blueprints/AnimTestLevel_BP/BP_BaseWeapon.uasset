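; BP_BaseWeapon is a base weapon Blueprint in the animation test level, built around a skeletal mesh.
; On BeginPlay it stores an aim baseline offset from the world-space distance between the mesh's Root and Sight sockets.
; Shoot plays the fire montage on the mesh.
; FirePressed only tests for an empty magazine and does nothing further, so it does not trigger Shoot.
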(event `self.ReceiveBeginPlay`
  (set `self.AimBaselineOffset` (- (`KismetAnimationLibrary.K2_DistanceBetweenTwoSocketsAndMapRange` (`self.SkeletalMesh`) "Root" "RTS_World" "Sight" "RTS_World") 0.0)))

(event `/Game/Blueprints/AnimTestLevel_BP/BPI_BaseWeapon.FirePressed`
  (if (== (`self.BulletsInMag`) 0)
    _))

(event `Shoot`
  (`|PlayMontage` (`self.SkeletalMesh`) "/Game/Animations/Rifle/A_AR_Fire_M.A_AR_Fire_M"))

(fn `UserConstructionScript`)